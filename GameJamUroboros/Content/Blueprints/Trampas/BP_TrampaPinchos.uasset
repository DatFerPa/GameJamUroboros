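; BP_TrampaPinchos is a hidden, one-shot spike trap that kills the player.
; On BeginPlay it hides the skeletal mesh, disables its collision and that of PasoParaJugador, and stores all PlayerStart actors, unused in these graphs.
; When a BP_Player overlaps the Trigger, it calls Die on the player, reveals the mesh, enables both collisions and disables the Trigger, leaving the sprung trap solid.
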(event OnComponentBeginOverlap(Trigger)
  (params (OverlappedComponent :type Primitive%20Component%20Object%20Reference) (OtherActor :type Actor%20Object%20Reference) (OtherComp :type Primitive%20Component%20Object%20Reference) (OtherBodyIndex :type Integer) (bFromSweep :type Boolean) (SweepResult :type Hit%20Result%20Structure%20%28by%20ref%29))
  (bind _skeletalmesh (Variables|Default|GetSkeletalMesh))
  (bind _asbp_player (Utilities|Casting|CastToBP_Player OtherActor))
  (Default|Die _asbp_player)
  (Rendering|SetVisibility _skeletalmesh true false)
  (Collision|SetCollisionEnabled _skeletalmesh "QueryAndPhysics")
  (Collision|SetCollisionEnabled (Variables|Default|GetPasoParaJugador) "QueryAndPhysics")
  (Collision|SetCollisionEnabled (Variables|Default|GetTrigger) "NoCollision"))

(event EventBeginPlay
  (bind _skeletalmesh (Variables|Default|GetSkeletalMesh))
  (Rendering|SetVisibility _skeletalmesh false false)
  (Collision|SetCollisionEnabled _skeletalmesh "NoCollision")
  (Collision|SetCollisionEnabled (Variables|Default|GetPasoParaJugador) "NoCollision")
  (bind _outactors (Actor|GetAllActorsOfClass "/Script/Engine.PlayerStart"))
  (Variables|Default|SetPlayerStarts _outactors))

(event Collision|EventActorBeginOverlap
  (params (OtherActor :type Actor%20Object%20Reference)))

(event EventTick
  (params (DeltaSeconds :type Float%20%28single-precision%29)))

(fn ConstructionScript)