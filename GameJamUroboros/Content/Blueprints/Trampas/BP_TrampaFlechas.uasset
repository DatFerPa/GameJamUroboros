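; BP_TrampaFlechas is an arrow trap that automatically fires BP_Flecha projectiles at a fixed interval.
; On BeginPlay, a DoOnce fires the first arrow immediately and starts a looping timer on DispararFlecha at the RatioDisparo interval, alongside a delayed gate reset.
; Each shot spawns the arrow at the Arrow component's world transform with the trap as owner.
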(event Custom|DispararFlecha
  (Game|SpawnActorfromClass "/Game/Blueprints/Trampas/BP_Flecha.BP_Flecha_C" (Transformation|GetWorldTransform (Variables|Default|GetArrow)) "Undefined" self 0))

(event EventBeginPlay
  (Utilities|FlowControl|DoOnce false :!label _label
    (:Completed
      (Utilities|FlowControl|Sequence
        (:then_0
          (Utilities|FlowControl|Delay (Variables|Default|GetRatioDisparo))
          (goto _label Reset))
        (:then_1
          (CallFunction|DispararFlecha)
          (Utilities|Time|SetTimerbyEvent (delegate Custom|DispararFlecha) (Variables|Default|GetRatioDisparo) true))))))

(event Collision|EventActorBeginOverlap
  (params (OtherActor :type Actor%20Object%20Reference)))

(event EventTick
  (params (DeltaSeconds :type Float%20%28single-precision%29)))

(fn ConstructionScript)