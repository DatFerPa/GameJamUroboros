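; Enemy that guards its spawn point, kills the player on contact and can be neutralized with bait.
; A control zone overlap flags player or bait presence; Tick sweeps the mesh along X toward bait first, then the player, otherwise back to spawn.
; Touching bait with the damage collider calls Comer, which shifts the actor on Y, turns it, turns off damage collision and disables movement.
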(event OnComponentBeginOverlap(controlZone)
  (params (OverlappedComponent :type Primitive%20Component%20Object%20Reference) (OtherActor :type Actor%20Object%20Reference) (OtherComp :type Primitive%20Component%20Object%20Reference) (OtherBodyIndex :type Integer) (bFromSweep :type Boolean) (SweepResult :type Hit%20Result%20Structure%20%28by%20ref%29))
  ;[1 1 1] Check player in control zone
  (Utilities|Casting|CastToBP_Bait OtherActor
    (:then
      (Variables|Default|SetBaitInRange true))
    (:CastFailed
      (Utilities|Casting|CastToBP_Player OtherActor)
      (Variables|Default|SetplayerInRange true))))

(event OnComponentEndOverlap(controlZone)
  (params (OverlappedComponent :type Primitive%20Component%20Object%20Reference) (OtherActor :type Actor%20Object%20Reference) (OtherComp :type Primitive%20Component%20Object%20Reference) (OtherBodyIndex :type Integer))
  ;[1 1 1] Check player in control zone
  (Utilities|Casting|CastToBP_Bait OtherActor
    (:then
      (Variables|Default|SetBaitInRange false))
    (:CastFailed
      (Utilities|Casting|CastToBP_Player OtherActor)
      (Variables|Default|SetplayerInRange false))))

(event OnComponentBeginOverlap(damageCollider)
  (params (OverlappedComponent :type Primitive%20Component%20Object%20Reference) (OtherActor :type Actor%20Object%20Reference) (OtherComp :type Primitive%20Component%20Object%20Reference) (OtherBodyIndex :type Integer) (bFromSweep :type Boolean) (SweepResult :type Hit%20Result%20Structure%20%28by%20ref%29))
  ;[1 1 1] DamageCollider
  (bind _asbp_player (Utilities|Casting|CastToBP_Player OtherActor)
    (:then
      (Default|Die _asbp_player))
    (:CastFailed
      (Utilities|Casting|CastToBP_Bait OtherActor)
      (CallFunction|Comer))))

(event EventBeginPlay
  ;[1 1 1] Begin play
  (Variables|Default|SetspawnPoint (Transformation|GetWorldLocation (Variables|Default|GetMesh))))

(event EventTick
  (params (DeltaSeconds :type Float%20%28single-precision%29))
  (if (not (Variables|Default|GetDisabled))
    (if (Variables|Default|GetBaitInRange)
      (bind _returnvalue (Actor|GetActorOfClass "/Game/Blueprints/BP_Bait.BP_Bait_C"))
      (if (< (.x (Transformation|GetActorLocation _returnvalue)) (.x (Transformation|GetWorldLocation (Variables|Default|GetMesh))))
        (Variables|Default|SetmovDirection "-1.000000, 0, 0")
        (else
          (Variables|Default|SetmovDirection "1.000000, 0, 0")))
      (Transformation|AddWorldOffset (Variables|Default|GetMesh) (* (Variables|Default|GetmovDirection) (* DeltaSeconds (Variables|Default|Getspeed))) true false)
      (elif (Variables|Default|GetplayerInRange)
        (if (< (.x (Transformation|GetActorLocation (Game|Player|GetPlayerPawn 0))) (.x (Transformation|GetWorldLocation (Variables|Default|GetMesh))))
          (Variables|Default|SetmovDirection "-1.000000, 0, 0")
          (else
            (Variables|Default|SetmovDirection "1.000000, 0, 0")))
        (Transformation|AddWorldOffset (Variables|Default|GetMesh) (* (Variables|Default|GetmovDirection) (* DeltaSeconds (Variables|Default|Getspeed))) true false)
        (elif (Math|Vector|NotEqual(Vector) (Transformation|GetWorldLocation (Variables|Default|GetMesh)) (Variables|Default|GetspawnPoint) 0.0001)
          (if (< (.x (Transformation|GetWorldLocation (Variables|Default|GetMesh))) (.x (Variables|Default|GetspawnPoint)))
            (Variables|Default|SetmovDirection "1.000000, 0, 0")
            (else
              (Variables|Default|SetmovDirection "-1.000000, 0, 0")))
          (Transformation|AddWorldOffset (Variables|Default|GetMesh) (* (Variables|Default|GetmovDirection) (* DeltaSeconds (Variables|Default|Getspeed))) true false))))))

(fn ConstructionScript)

(fn Comer
  (bind _returnvalue (Transformation|GetActorLocation))
  (bind _returnvalue_2 (Transformation|GetActorRotation))
  (Transformation|SetActorLocation (Math|Vector|MakeVector (.x _returnvalue) (+ (.y _returnvalue) (Variables|Default|GetYDisplacement)) (.z _returnvalue)) false false)
  (Transformation|SetActorRotation (Math|Rotator|MakeRotator (.roll _returnvalue_2) (.pitch _returnvalue_2) -9e+01))
  (Collision|SetCollisionEnabled (Variables|Default|GetdamageCollider) "NoCollision")
  (Variables|Default|SetDisabled true)
  (Development|PrintString "Comer finalizado"))