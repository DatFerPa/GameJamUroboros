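; BP_Interact is an interactable magic stone that shows a text prompt while its trigger is overlapped and it is active.
; It enables input from player controller 0, and pressing Interact while the player is flagged inside the trigger calls Activate.
; Activate re-enables every BP_Interact actor with the enabled material, then disables itself and hides its prompt, leaving only the last-used stone inactive.
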(event OnComponentBeginOverlap(Trigger)
  (params (OverlappedComponent :type Primitive%20Component%20Object%20Reference) (OtherActor :type Actor%20Object%20Reference) (OtherComp :type Primitive%20Component%20Object%20Reference) (OtherBodyIndex :type Integer) (bFromSweep :type Boolean) (SweepResult :type Hit%20Result%20Structure%20%28by%20ref%29))
  (if (Variables|Default|GetInteractActive)
    (Rendering|SetVisibility (Variables|Default|GetTextToShow) true false)
    (Variables|Default|SetPlayerInTrigger true)))

(event OnComponentEndOverlap(Trigger)
  (params (OverlappedComponent :type Primitive%20Component%20Object%20Reference) (OtherActor :type Actor%20Object%20Reference) (OtherComp :type Primitive%20Component%20Object%20Reference) (OtherBodyIndex :type Integer))
  (Rendering|SetVisibility (Variables|Default|GetTextToShow) false false)
  (Variables|Default|SetPlayerInTrigger false))

(event EventBeginPlay
  (Input|EnableInput (Game|GetPlayerController 0)))

(event Input|ActionEvents|InputActionInteract
  (params (Key :type Key%20Structure :default "None"))
  (:Pressed
    (if (Variables|Default|GetPlayerInTrigger)
      (CallFunction|Activate))))

(fn ConstructionScript)

(fn Activate
  ;[1 1 1] Activate
  (bind _outactors (Actor|GetAllActorsOfClass "BP_Interact_C"))
  (for _array_element _outactors
    (Variables|BP_Interact_C|SetInteractActive _array_element true)
    (Rendering|Material|SetMaterial (Variables|BP_Interact_C|GetStaticMesh _array_element) 0 "/Game/beffio/Medieval_Kingdom/Content/Materials/Materials_Instances/MagicStone/MI_Magic_Stone_Enable.MI_Magic_Stone_Enable"))
  (Variables|Default|SetInteractActive false)
  (Rendering|Material|SetMaterial (Variables|Default|GetStaticMesh) 0 "/Game/beffio/Medieval_Kingdom/Content/Materials/Materials_Instances/MagicStone/MI_Magic_Stone_Disable.MI_Magic_Stone_Disable")
  (Rendering|SetVisibility (Variables|Default|GetTextToShow) false false))