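; Player character that moves along the X axis, jumps, and drinks potions that kill it.
; Potion 1 leaves a BP_Rock at its position after a smoke effect and Potion 2 triggers an explosion effect, while Potions 3 and 4 only print text.
; Die hides the character, stops movement and dims the directional light, then Respawnear teleports it to the first PlayerStart and restores them, clearing the flag that blocks repeat potion use.
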(event Custom|Respawnear
  ;[1 1 1] Respawn
  (Utilities|FlowControl|Delay 2.0)
  (bind _returnvalue (Transformation|Teleport (Transformation|GetActorLocation (Utilities|Array|Get(acopy) (Variables|Default|GetPlayerStart))) "0, 0, 0"))
  (if _returnvalue
    (Variables|Default|SetPotionFlag false)
    (Development|SetHiddeninGame (Variables|Collision|GetCapsuleComponent) false false)
    (Components|Activation|SetActive (Variables|Character|GetCharacterMovement) true false)
    (Rendering|Components|Light|SetIntensity (Variables|/Script/Engine.Light|GetLightComponent (Utilities|Array|Get(acopy) (Variables|Default|GetLight))) 1e+01)))

(event EventBeginPlay
  ;[1 1 1] Begin Play
  (bind _outactors (Actor|GetAllActorsOfClass "/Script/Engine.PlayerStart"))
  (Variables|Default|SetPlayerStart _outactors)
  (bind _outactors_2 (Actor|GetAllActorsOfClass "/Script/Engine.DirectionalLight"))
  (Variables|Default|SetLight _outactors_2))

(event Collision|EventActorBeginOverlap
  (params (OtherActor :type Actor%20Object%20Reference)))

(event Input|ActionEvents|InputActionJump
  (params (Key :type Key%20Structure :default "None"))
  ;[1 1 1] Jump Button
  (:Pressed
    (Character|Jump))
  (:Released
    (Character|StopJumping)))

(event Input|ActionEvents|InputActionPotion1
  (params (Key :type Key%20Structure :default "None"))
  ;[1 1 1] Potions
  (:Pressed
    (Development|PrintString "Pocion de convertir en piedra")
    (if (not (Variables|Default|GetPotionFlag))
      (Variables|Default|SetPotionFlag true)
      (bind _returnvalue (Game|SpawnActorfromClass "/Game/StarterContent/Blueprints/Blueprint_Effect_Steam.Blueprint_Effect_Steam_C" (Transformation|GetWorldTransform (Variables|Collision|GetCapsuleComponent)) "AlwaysSpawn" 0 0))
      (bind _output_get (Variables|Default|SetSmoke _returnvalue))
      (Transformation|SetActorRotation _output_get "80.000000, 0, 0")
      (Transformation|SetActorLocation (Variables|Default|GetSmoke) (Math|Vector|MakeVector (+ (.x (Transformation|GetActorLocation (Variables|Default|GetSmoke))) 5e+01) (.y (Transformation|GetActorLocation (Variables|Default|GetSmoke))) (- (.z (Transformation|GetActorLocation (Variables|Default|GetSmoke))) 1.2e+02)) false false)
      (Transformation|AttachActorToActor (Variables|Default|GetSmoke) self "None" "KeepWorld" "KeepWorld" "KeepWorld" true)
      (Utilities|FlowControl|Delay 1.0)
      (Game|SpawnActorfromClass "/Game/Blueprints/BP_Rock.BP_Rock_C" (Transformation|GetWorldTransform (Variables|Collision|GetCapsuleComponent)) "AlwaysSpawn" 0 0)
      (Actor|DestroyActor (Variables|Default|GetSmoke))
      (CallFunction|Die))))

(event Input|ActionEvents|InputActionPotion2
  (params (Key :type Key%20Structure :default "None"))
  ;[1 1 1] Potions
  (:Pressed
    (Development|PrintString "Pocion de explotar")
    (if (not (Variables|Default|GetPotionFlag))
      (Variables|Default|SetPotionFlag true)
      (Rendering|SetVisibility (Variables|Default|GetCube) false false)
      (bind _returnvalue (Game|SpawnActorfromClass "/Game/StarterContent/Blueprints/Blueprint_Effect_Explosion.Blueprint_Effect_Explosion_C" (Transformation|GetWorldTransform (Variables|Collision|GetCapsuleComponent)) "AlwaysSpawn" 0 0))
      (Variables|Default|SetExplotion _returnvalue)
      (Transformation|AttachActorToActor (Variables|Default|GetExplotion) self "None" "KeepWorld" "KeepWorld" "KeepWorld" true)
      (Utilities|FlowControl|Delay 1.0)
      (Actor|DestroyActor (Variables|Default|GetExplotion))
      (CallFunction|Die)
      (Rendering|SetVisibility (Variables|Default|GetCube) true false))))

(event Input|ActionEvents|InputActionPotion3
  (params (Key :type Key%20Structure :default "None"))
  ;[1 1 1] Potions
  (:Pressed
    (Development|PrintString "Pocion 3")))

(event Input|ActionEvents|InputActionPotion4
  (params (Key :type Key%20Structure :default "None"))
  ;[1 1 1] Potions
  (:Pressed
    (Development|PrintString "Pocion 4")))

(event Input|AxisEvents|InputAxisMoveRight
  (params (AxisValue :type Float%20%28single-precision%29))
  ;[1 1 1] Movement
  (Pawn|Input|AddMovementInput "1.000000, 0, 0" AxisValue false))

(fn ConstructionScript)

(fn Die
  (Development|SetHiddeninGame (Variables|Collision|GetCapsuleComponent) true true)
  (Components|Activation|SetActive (Variables|Character|GetCharacterMovement) false false)
  (Rendering|Components|Light|SetIntensity (Variables|/Script/Engine.Light|GetLightComponent (Utilities|Array|Get(acopy) (Variables|Default|GetLight))) 0.02)
  (CallFunction|Respawnear))